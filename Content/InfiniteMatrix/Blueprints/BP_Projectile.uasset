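; BP_Projectile is a projectile that destroys enemies and awards score to the player.
; Each Tick it looks up BP_Player actors and moves along world X with a swept offset at twice their ForwardSpeed, scaled by delta time.
; When its Box overlaps a BP_Enemy, it increments the player's Score and destroys both the enemy and itself.
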(event OnComponentBeginOverlap(Box)
  (params (OverlappedComponent :type Primitive%20Component%20Object%20Reference) (OtherActor :type Actor%20Object%20Reference) (OtherComp :type Primitive%20Component%20Object%20Reference) (OtherBodyIndex :type Integer) (bFromSweep :type Boolean) (SweepResult :type Hit%20Result%20Structure%20%28by%20ref%29))
  (bind _asbp_enemy (Utilities|Casting|CastToBP_Enemy OtherActor))
  (bind _outactors (Actor|GetAllActorsOfClass "/Game/InfiniteMatrix/Blueprints/BP_Player.BP_Player_C"))
  (for _array_element _outactors
    (Variables|/Game/InfiniteMatrix/Blueprints/BP_Player.BP_Player_C|SetScore _array_element (+ (Variables|/Game/InfiniteMatrix/Blueprints/BP_Player.BP_Player_C|GetScore _array_element) 1))
    (Actor|DestroyActor _asbp_enemy)
    (Actor|DestroyActor)))

(event EventBeginPlay)

(event Collision|EventActorBeginOverlap
  (params (OtherActor :type Actor%20Object%20Reference)))

(event EventTick
  (params (DeltaSeconds :type Float%20%28single-precision%29))
  (bind _outactors (Actor|GetAllActorsOfClass "/Game/InfiniteMatrix/Blueprints/BP_Player.BP_Player_C"))
  (for _array_element _outactors
    (Transformation|AddActorWorldOffset (Math|Vector|MakeVector (* DeltaSeconds (* (Variables|/Game/InfiniteMatrix/Blueprints/BP_Player.BP_Player_C|GetForwardSpeed _array_element) 2.0)) 0.0 0.0) true)))

(fn ConstructionScript)